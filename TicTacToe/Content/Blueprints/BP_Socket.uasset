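; BP_Socket is a board cell for what appears to be tic-tac-toe, holding an empty, X or O state.
; Three functions set State and toggle the XMark and ZeroMark components to match.
; The two show functions reveal only their own mark, while HideMarksAndSetEmptyState hides both.
; Event graph logic deriving visibility from State is disconnected, so changes happen only through function calls.
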(event EventBeginPlay)

(event Collision|EventActorBeginOverlap
  (params (OtherActor :type Actor%20Object%20Reference)))

(event EventTick
  (params (DeltaSeconds :type Float%20%28single-precision%29)))

(fn ConstructionScript)

(fn ShowandSetXMark
  (Rendering|SetVisibility (Variables|Default|GetXMark) true false)
  (Variables|Default|SetState "XMark"))

(fn ShowandSetZeroMark
  (Rendering|SetVisibility (Variables|Default|GetZeroMark) true false)
  (Variables|Default|SetState "OMark"))

(fn HideMarksandSetEmptyState
  (Rendering|SetVisibility (Variables|Default|GetXMark) false false)
  (Rendering|SetVisibility (Variables|Default|GetZeroMark) false false)
  (Variables|Default|SetState "Empty"))