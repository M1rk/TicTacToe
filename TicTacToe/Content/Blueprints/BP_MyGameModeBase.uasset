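; Game mode for a tic-tac-toe match between the player and a MiniMax AI, with a menu widget for results.
; BeginPlay shows the menu and builds OriginBoard from BP_Socket actors ordered by Index.
; A click on an empty socket places the player's mark, then after a delay MiniMax picks the AI's move.
; Only AI wins and full-board ties are checked; either switches input to UI only.
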(event EventBeginPlay
  (bind _returnvalue (Game|GetPlayerController 0))
  ;[1 1 1] Устанавливаем дефолтные значения фишек
  (Variables|Default|SetPlayerMark "X")
  (Variables|Default|SetAIMark "0")
  ;[1 1 1] Создаем виджет, кладём ссылку в переменную,добавляем на экран,включаем ввод
  (bind _returnvalue_2 (UserInterface|CreateWidget "/Game/UI/WGT_Menu.WGT_Menu_C"))
  (Variables|Default|SetMenuWidget _returnvalue_2)
  (UserInterface|Viewport|AddtoViewport _returnvalue_2 0)
  (Input|EnableInput _returnvalue)
  (Variables|/Script/Engine.PlayerController|SetbShowMouseCursor _returnvalue true)
  ;[1 1 1] Наполняем массив OriginBoard сокетами игрового поля
  (bind _outactors (Actor|GetAllActorsOfClass "/Game/Blueprints/BP_Socket.BP_Socket_C"))
  (for _index (range 0 8)
    (bind _array_element (Utilities|Array|ForEachLoopwithBreak _outactors)
      (:LoopBody
        (if (== (Variables|/Script/TicTacToe.Socket|Getindex _array_element) _index)
          (Utilities|Array|Add (Variables|Default|GetOriginBoard) _array_element))))))

(event Input|ActionEvents|InputActionLeftMouseClick
  (params (Key :type Key%20Structure))
  (bind _returnvalue (Game|GetPlayerController 0))
  (bind _array (Utilities|Array|MakeArray "ObjectTypeQuery1" "ObjectTypeQuery2" "ObjectTypeQuery4"))
  (bind _menuwidget (Variables|Default|GetMenuWidget))
  (bind _aimark (Variables|Default|GetAIMark))
  (bind (_hitresult _returnvalue_2) (Class|PlayerController|GetHitResultUnderCursorforObjects _returnvalue _array true))
  (:Pressed
    ;[1 1 1] Получаем актора по клику мыши,проверяем на очередность хода и на свободное место для хода
    (if _returnvalue_2
      (bind _asbp_socket (Utilities|Casting|CastToBP_Socket (.HitActor (Collision|BreakHitResult _hitresult))))
      (if (Utilities|Enum|Equal(Enum) (Variables|/Script/TicTacToe.Socket|GetState _asbp_socket) "Empty")
        (if (Utilities|Enum|Equal(Enum) (Variables|Default|GetTurnState) "PlayerTurn")
          (Audio|PlaySound2D "/Game/Sounds/S_Switch19-intermed-5229_hifi.S_Switch19-intermed-5229_hifi" 1.0 1.0 0.0 0 0)
          ;[1 1 1] В зависимости от фишки игрока проявляем нужный меш и меняем состояние сокета
          (switch string (Variables|Default|GetPlayerMark)
            (:X
              (Default|ShowandSetXMark _asbp_socket)
              ;[1 1 1] Инкрементируем количество ходов,выставляем очередь хода ИИ
              (Variables|Default|SetMovesCount (+ (Variables|Default|GetMovesCount) 1))
              (Variables|Default|SetTurnState "AITurn")
              ;[1 1 1] проверка на заполненность всего поля
              (CallFunction|CheckforEmptySlots)
              (if (Variables|Default|GetIsBoardFilled)
                ;[1 1 1] В случае, если свободных полей больше нет, показываем сообщение о ничьей
                (Widget|SetVisibility (Variables|/Game/UI/WGT_Menu.WGT_Menu_C|GetTieTEXT (Variables|Default|GetMenuWidget)) "Visible")
                (Input|SetInputModeUIOnly (Game|GetPlayerController 0) 0 "DoNotLock")
                (else
                  (Utilities|FlowControl|Delay 1.2)
                  ;[1 1 1] Непосредственно функция алгоритма МиниМакс, возвращающая структуру с индексом и весом лучшего хода
                  (bind _returnvalue_3 (Class|MyGameModeBase|MiniMax (Variables|Default|GetOriginBoard) _aimark))
                  ;[1 1 1] Инкрементируем счетчик ходов, показываем фишку,меняем стейт сокета
                  (Default|ShowandSetZeroMark (Utilities|Array|Get(acopy) (Variables|Default|GetOriginBoard) (.index (Utilities|Struct|BreakMovement _returnvalue_3))))
                  (Variables|Default|SetMovesCount (+ (Variables|Default|GetMovesCount) 1) :!label _label)
                  (Audio|PlaySound2D "/Game/Sounds/S_Switch19-intermed-5239_hifi.S_Switch19-intermed-5239_hifi" 1.0 1.0 0.0 0 0)
                  ;[1 1 1] Устанавливаем очередь хода игрока,проверяем на победу ИИ
                  (Variables|Default|SetTurnState "PlayerTurn")
                  (bind _returnvalue_4 (Class|MyGameModeBase|Winning (Variables|Default|GetOriginBoard) (Variables|Default|GetAIMark)))
                  (if _returnvalue_4
                    ;[1 1 1] В случае победы ИИ показываем текст "Проигрыш"
                    (Widget|SetVisibility (Variables|/Game/UI/WGT_Menu.WGT_Menu_C|GetLoseTEXT _menuwidget) "Visible")
                    (Input|SetInputModeUIOnly (Game|GetPlayerController 0) 0 "DoNotLock" :!label _label_2)
                    (else
                      ;[1 1 1] В случае, если слотов больше нет, показываем сообщение "ничья"
                      (CallFunction|CheckforEmptySlots)
                      (if (Variables|Default|GetIsBoardFilled)
                        (Widget|SetVisibility (Variables|/Game/UI/WGT_Menu.WGT_Menu_C|GetTieTEXT _menuwidget) "Visible")
                        (goto _label_2)))))))
            (:0
              (Default|ShowandSetZeroMark _asbp_socket)
              ;[1 1 1] Инкрементируем количество ходов,выставляем очередь хода ИИ
              (Variables|Default|SetMovesCount (+ (Variables|Default|GetMovesCount) 1))
              (Variables|Default|SetTurnState "AITurn")
              ;[1 1 1] проверка на заполненность всего поля
              (CallFunction|CheckforEmptySlots)
              (if (Variables|Default|GetIsBoardFilled)
                ;[1 1 1] В случае, если свободных полей больше нет, показываем сообщение о ничьей
                (Widget|SetVisibility (Variables|/Game/UI/WGT_Menu.WGT_Menu_C|GetTieTEXT (Variables|Default|GetMenuWidget)) "Visible")
                (Input|SetInputModeUIOnly (Game|GetPlayerController 0) 0 "DoNotLock")
                (else
                  (Utilities|FlowControl|Delay 1.2)
                  (bind _returnvalue_5 (Class|MyGameModeBase|MiniMax (Variables|Default|GetOriginBoard) _aimark))
                  (Default|ShowandSetXMark (Utilities|Array|Get(acopy) (Variables|Default|GetOriginBoard) (.index (Utilities|Struct|BreakMovement _returnvalue_5))))
                  (goto _label))))))))))

(fn ConstructionScript)

(fn CheckforEmptySlots
  ;[1 1 1] Проверка на заполненность всех полей в игре
  (Variables|Default|SetIsBoardFilled true)
  (bind _array_element (Utilities|Array|ForEachLoopwithBreak (Variables|Default|GetOriginBoard) :!label _label)
    (:LoopBody
      (if (Utilities|Enum|Equal(Enum) (Variables|/Script/TicTacToe.Socket|GetState _array_element) "Empty")
        (Variables|Default|SetIsBoardFilled false)
        (goto _label Break)))))